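; Test actor that demonstrates One Euro filtering by following a Source actor that it jitters with random noise.
; Each tick it sets Source to its starting transform plus random location and rotation offsets.
; It then feeds Source's transform through a transform filter and applies the smoothed location and rotation with raw scale to itself.
; An offset captured at BeginPlay keeps it visually apart from Source for comparison.
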(event `self.ReceiveBeginPlay`
  (`self.Init`))

(event `self.ReceiveTick`
  (params (DeltaSeconds :type "Float (single-precision)"))
  (`self.ApplyNoiseToSource`)
  (`self.FilterThenApplySourceTransform`))

(fn `ApplyNoiseToSource`
  (bind (_startingtransform_location _startingtransform_rotation) (`KismetMathLibrary.BreakTransform` (`self.StartingTransform`)))
  ;[0.1146 0.1104 0.1043] Applying random offset to location and rotation of the Source actor, in order to simulate a noisy movement
  (`self.K2_SetActorTransform` (`self.Source`) (`KismetMathLibrary.MakeTransform` (+ (* (`KismetMathLibrary.RandomUnitVector`) 20.0) _startingtransform_location) (`KismetMathLibrary.ComposeRotators` _startingtransform_rotation (* (`KismetMathLibrary.RandomRotator` true) 0.05))) false false))

(fn `FilterThenApplySourceTransform`
  (`|ExecutionSequence`
    (:`then_0`
      ;[0.2916 0.5746 1] Retrieving the transform of the ActorToFollow, and passing it to the OneEuroFilter, which will filter the whole Transform
      (`OneEuroFilterBPFunctionLibrary.SetTransformValue` (`self.TransformFilter`) (`self.GetTransform` (`self.Source`)))
      ;[1 0.6144 0.1961] Getting the filtered transform from the OneEuroFilter variable, and applying it to the actor. Note how we are bypassing scale.
      ; This will give us filtered location and rotation, and raw scale.
      (`self.K2_SetActorTransform` (`.Filtered` (`OneEuroFilterBPFunctionLibrary.GetTransformValue` (`self.TransformFilter`)))))
    (:`then_1`
      ;[1 1 1] ADDITIONAL: Keeping the actor distant from the ActorToFollow.
      ; This makes it easier to look at the movements of the filtered object.
      ; This is just for display.
      (`self.K2_AddActorWorldOffset` (`self.LocationOffset`)))))

(fn `Init`
  (`|ExecutionSequence`
    (:`then_0`
      ;[1 1 1] Storing starting Transform for object to follow (Source actor).
      ; This information will be used to make it bounce around in a noisy way
      (set `self.StartingTransform` (`self.GetTransform` (`self.Source`))))
    (:`then_1`
      ;[1 1 1] Computing vector from Source actor to this object, so that we keep them at the same distance.
      (set `self.LocationOffset` (- (`self.K2_GetActorLocation`) (`self.K2_GetActorLocation` (`self.Source`)))))))

(fn `UserConstructionScript`)